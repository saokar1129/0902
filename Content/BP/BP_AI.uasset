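; Zombie AI character Blueprint that wanders, chases and attacks the player character (BP_person), and takes damage.
; BeginPlay loops random nearby moves with short random pauses.
; PawnSensing sightings trigger a move to the player, then an attack montage throttled by a flag and a DoOnce reset after a delay.
; 受傷 (take damage) subtracts health and plays a hit montage, plus a death montage at zero, without stopping the AI.
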(event `self.ReceiveBeginPlay`
  (`|AIMoveTo` self (`NavigationSystemV1.K2_GetRandomReachablePointInRadius` (`SceneComponent.K2_GetComponentLocation` (`self.Mesh`)) 500.0 null null) null :!label _label
    (:`OnSuccess`
      _)
    (:`OnFail`
      _))
  (`KismetSystemLibrary.Delay` (`KismetMathLibrary.RandomFloatInRange` 1.0 5.0))
  (goto _label))

(event `self.PawnSensing.OnSeePawn`
  (params (Pawn :type "Pawn Object Reference"))
  (if (not (`self.攻擊玩家`))
    (bind _asbp_person (cast `/Game/BP/BP_person` Pawn))
    (`|AIMoveTo` self (0.0 0.0 0.0) _asbp_person
      (:`OnSuccess`
        (`/Engine/EditorBlueprintResources/StandardMacros.DoOnce` false :!label _label_2
          (:`Completed`
            (`|PlayMontage` (`self.Mesh`) "/Game/animation/AI/Zombie_Attack_Montage.Zombie_Attack_Montage"
              (:`then`
                (set `self.攻擊玩家` true))
              (:`OnCompleted`
                (set `self.攻擊玩家` false)
                (`KismetSystemLibrary.Delay` 0.4)
                (goto _label_2 :!via `Reset`)))))))))

(fn `UserConstructionScript`)

(fn `受傷`
  (params (`傷害值` :type "Float (double-precision)"))
  (set `self.血量` (- (`self.血量`) `傷害值`))
  (`self.PlayAnimMontage` self "/Game/animation/AI/hit_AI_Montage.hit_AI_Montage" 1.0 "None")
  (if (<= (`self.血量`) 0.0)
    (`self.PlayAnimMontage` self "/Game/animation/AI/dead_AI_Montage.dead_AI_Montage" 1.0 "None")))